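; Voxel block spawner that builds an instanced static mesh component per block type and places blocks as instances on a 100-unit grid.
; On BeginPlay, ScanBlocks fills MeshArray through CreateMeshes, assigning six face materials or reusing Top when Bottom is unset, then PlaceBlock spawns one block.
; World-array and chunk-string parsing is present but disconnected.
; The X key only prints a loading message.
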(event `self.ReceiveBeginPlay`
  (set `self.keyPress` 0)
  (`self.EnableInput` (`GameplayStatics.GetPlayerController` 0))
  (`self.scanBlocks`)
  (`self.placeBlock` (`|GetArrayItem` (`self.meshArray`) 8)))

(event `Key|X`
  (params (Key :type "Key Structure"))
  (:`Pressed`
    (for _index (range 5)
      (`KismetSystemLibrary.PrintString` "LOADING CHUNK...."))))

(event `Key|P`
  (params (Key :type "Key Structure")))

(fn `checkBlock`
  (params (`Array Element` :type String) (block :type "InstancedStaticMeshComponent Object Reference") (index :type Integer))
  (if (`KismetStringLibrary.EqualEqual_StrStr` `Array Element` (`KismetStringLibrary.Conv_IntToString` index))
    (if (== index 0)
      (bind _output_get (set `self.x` (+ (stale _output_get) 1)))
      (else
        (`self.placeBlock` block (`self.x`) (`self.y`) (`self.z`))))))

(fn `createMeshes`
  (params (Top :type "MaterialInterface Object Reference") (Bottom :type "MaterialInterface Object Reference") (Front :type "MaterialInterface Object Reference") (Back :type "MaterialInterface Object Reference") (Right :type "MaterialInterface Object Reference") (Left :type "MaterialInterface Object Reference") (id :type Integer))
  (locals (XTop :type "MaterialInterface Object Reference") (XBottom :type "MaterialInterface Object Reference") (XRight :type "MaterialInterface Object Reference") (XLeft :type "MaterialInterface Object Reference") (XFront :type "MaterialInterface Object Reference") (XBack :type "MaterialInterface Object Reference"))
  (set `local.XTop` Top)
  (`/Engine/EditorBlueprintResources/StandardMacros.IsValid` Bottom
    (:`Is Valid`
      (set `local.XBottom` Bottom)
      (set `local.XRight` Right)
      (set `local.XLeft` Left)
      (set `local.XFront` Front)
      (set `local.XBack` Back))
    (:`Is Not Valid`
      (set `local.XBottom` Top)
      (set `local.XRight` Top)
      (set `local.XLeft` Top)
      (set `local.XFront` Top)
      (set `local.XBack` Top)))
  (if (== (`self.index`) id)
    (bind _returnvalue (`AddComponent|NODE_AddInstancedStaticMeshComponent-5` :`bManualAttachment` true))
    (set `InstancedStaticMeshComponent.KeepInstanceBufferCPUAccess` false _returnvalue)
    (`SceneComponent.K2_AttachToComponent` _returnvalue (`self.DefaultSceneRoot`) "None" "KeepRelative" "KeepRelative" "KeepRelative" true)
    (`PrimitiveComponent.SetMaterial` _returnvalue 0 (`local.XRight`))
    (`PrimitiveComponent.SetMaterial` _returnvalue 1 (`local.XFront`))
    (`PrimitiveComponent.SetMaterial` _returnvalue 2 (`local.XBack`))
    (`PrimitiveComponent.SetMaterial` _returnvalue 3 (`local.XLeft`))
    (`PrimitiveComponent.SetMaterial` _returnvalue 4 (`local.XTop`))
    (`PrimitiveComponent.SetMaterial` _returnvalue 5 (`local.XBottom`))
    (`KismetArrayLibrary.Array_Add` (`self.meshArray`) _returnvalue)))

(fn `NewStuff`
  (params (Chunk :type Integer) (Index :type Integer)))

(fn `nextLayer`
  (params (Index :type Integer))
  (bind _mesharray (`self.meshArray`))
  (bind _output (`|GetArrayItem` (`self.worldArray`) Index))
  (for _index (range (`KismetArrayLibrary.Array_Length` _mesharray))
    (`/Engine/EditorBlueprintResources/StandardMacros.IncrementInt` (`self.newLineCounter`)
      (:`  `
        (`self.checkBlock` _output (`|GetArrayItem` _mesharray _index) _index))))
  (if (`KismetStringLibrary.EqualEqual_StrStr` _output "LINEBREAK")
    (`KismetSystemLibrary.PrintString` (`KismetStringLibrary.Conv_IntToString` (`self.newLineCounter`)))
    (set `self.newLineCounter` 0)
    (set `self.x` 0)
    (bind _output_get (set `self.y` (+ (stale _output_get) 1)))
    (elif (`KismetStringLibrary.EqualEqual_StrStr` _output "LAYERBREAK")
      (set `self.x` 0)
      (set `self.y` 0)
      (bind _output_get_2 (set `self.z` (+ (stale _output_get_2) 1))))))

(fn `placeBlock`
  (params (block :type "InstancedStaticMeshComponent Object Reference") (x :type Integer) (y :type Integer) (z :type Integer))
  (`InstancedStaticMeshComponent.AddInstance` block (`KismetMathLibrary.MakeTransform` (`KismetMathLibrary.MakeVector` (`KismetMathLibrary.Conv_IntToDouble` (* x 100)) (`KismetMathLibrary.Conv_IntToDouble` (* y 100)) (`KismetMathLibrary.Conv_IntToDouble` (* z 100))) (struct) (0.5 0.5 0.5)))
  (bind _output_get (set `self.x` (+ (stale _output_get) 1))))

(fn `scanBlocks`
  (locals (BlockArray :type "MaterialInterface Object Reference"))
  (for _index (range 59)
    (set `self.index` _index)
    (`self.createMeshes` null)
    (`self.createMeshes` null null null null null null 1)
    (`self.createMeshes` null null null null null null 2)
    (`self.createMeshes` null null null null null null 3)
    (`self.createMeshes` null null null null null null 4)
    (`self.createMeshes` null null null null null null 5)
    (`self.createMeshes` null null null null null null 6)
    (`self.createMeshes` null null null null null null 7)
    (`self.createMeshes` null null null null null null 8)
    (`self.createMeshes` null null null null null null 9)
    (`self.createMeshes` null null null null null null 10)
    (`self.createMeshes` null null null null null null 11)
    (`self.createMeshes` null null null null null null 12)
    (`self.createMeshes` null null null null null null 13)
    (`self.createMeshes` null null null null null null 14)
    (`self.createMeshes` null null null null null null 15)
    (`self.createMeshes` null null null null null null 16)
    (`self.createMeshes` null null null null null null 17)
    (`self.createMeshes` null null null null null null 18)
    (`self.createMeshes` null null null null null null 19)
    (`self.createMeshes` null null null null null null 20)
    (`self.createMeshes` null null null null null null 21)
    (`self.createMeshes` null null null null null null 22)
    (`self.createMeshes` null null null null null null 23)
    (`self.createMeshes` null null null null null null 24)
    (`self.createMeshes` null null null null null null 25)
    (`self.createMeshes` null null null null null null 26)
    (`self.createMeshes` null null null null null null 27)
    (`self.createMeshes` null null null null null null 28)
    (`self.createMeshes` null null null null null null 29)
    (`self.createMeshes` null null null null null null 30)
    (`self.createMeshes` null null null null null null 31)
    (`self.createMeshes` null null null null null null 32)
    (`self.createMeshes` null null null null null null 33)
    (`self.createMeshes` null null null null null null 34)
    (`self.createMeshes` null null null null null null 35)
    (`self.createMeshes` null null null null null null 36)
    (`self.createMeshes` null null null null null null 37)
    (`self.createMeshes` null null null null null null 38)
    (`self.createMeshes` null null null null null null 39)
    (`self.createMeshes` null null null null null null 40)
    (`self.createMeshes` null null null null null null 41)
    (`self.createMeshes` null null null null null null 42)
    (`self.createMeshes` null null null null null null 43)
    (`self.createMeshes` null null null null null null 44)
    (`self.createMeshes` null null null null null null 45)
    (`self.createMeshes` null null null null null null 46)
    (`self.createMeshes` null null null null null null 47)
    (`self.createMeshes` null null null null null null 48)
    (`self.createMeshes` null null null null null null 49)
    (`self.createMeshes` null null null null null null 50)
    (`self.createMeshes` null null null null null null 51)
    (`self.createMeshes` null null null null null null 52)
    (`self.createMeshes` null null null null null null 53)
    (`self.createMeshes` null null null null null null 54)
    (`self.createMeshes` null null null null null null 55)
    (`self.createMeshes` null null null null null null 56)
    (`self.createMeshes` null null null null null null 57)
    (`self.createMeshes` null null null null null null 58)
    (`self.createMeshes` null null null null null null 59)
    (`self.createMeshes` null null null null null null 60)
    (`self.createMeshes` null null null null null null 61)
    (`self.createMeshes` null null null null null null 62)
    (`self.createMeshes` null null null null null null 63)
    (`self.createMeshes` null null null null null null 64)))

(fn `SetSide`)

(fn `UserConstructionScript`)