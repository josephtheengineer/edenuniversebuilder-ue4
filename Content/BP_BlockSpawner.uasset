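; Block world spawner that builds a voxel level from a pipe-delimited converter file, world.out.
; On BeginPlay it creates one instanced static mesh component per block ID up to 58, with per-face materials falling back to top or front, then loads the file.
; Pressing X walks the tokens in two loops, adding grid-spaced instances for matching IDs.
; ID 0 leaves a gap, while LINEBREAK and LAYERBREAK tokens advance row and layer.
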(event `self.ReceiveBeginPlay`
  (set `self.keyPress` 0)
  (`self.EnableInput` (`GameplayStatics.GetPlayerController` 0))
  (`self.scanBlocks`))

(event `Key|X`
  (params (Key :type "Key Structure"))
  (bind _returnvalue (`KismetArrayLibrary.Array_Length` (`self.worldArray`)))
  (:`Pressed`
    (for _index (range (+ (/ (`KismetArrayLibrary.Array_Length` (`self.worldArray`)) 2) 1))
      (set `self.ForIndex` _index)
      (`self.nextLayer` (`self.ForIndex`) :!label _label))
    (for _index_2 (range (/ _returnvalue 2) _returnvalue)
      (set `self.ForIndex` _index_2)
      (goto _label))))

(event `Key|P`
  (params (Key :type "Key Structure")))

(fn `checkBlock`
  (params (`Array Element` :type String) (block :type "InstancedStaticMeshComponent Object Reference") (index :type Integer))
  (if (`KismetStringLibrary.EqualEqual_StrStr` `Array Element` (`KismetStringLibrary.Conv_IntToString` index))
    (if (== index 0)
      (bind _output_get (set `self.x` (+ (stale _output_get) 1)))
      (else
        (`self.placeBlock` block (`self.x`) (`self.y`) (`self.z`))))))

(fn `createMeshes`
  (params (Top :type "MaterialInterface Object Reference") (Bottom :type "MaterialInterface Object Reference") (Front :type "MaterialInterface Object Reference") (Back :type "MaterialInterface Object Reference") (Right :type "MaterialInterface Object Reference") (Left :type "MaterialInterface Object Reference") (id :type Integer))
  (locals (XTop :type "MaterialInterface Object Reference") (XBottom :type "MaterialInterface Object Reference") (XRight :type "MaterialInterface Object Reference") (XLeft :type "MaterialInterface Object Reference") (XFront :type "MaterialInterface Object Reference") (XBack :type "MaterialInterface Object Reference"))
  (set `local.XTop` Top)
  (`/Engine/EditorBlueprintResources/StandardMacros.IsValid` Bottom
    (:`Is Valid`
      (set `local.XBottom` Bottom))
    (:`Is Not Valid`
      (set `local.XBottom` Top)))
  (`/Engine/EditorBlueprintResources/StandardMacros.IsValid` Front
    (:`Is Valid`
      (set `local.XFront` Front)
      (`/Engine/EditorBlueprintResources/StandardMacros.IsValid` Back
        (:`Is Valid`
          (set `local.XBack` Back))
        (:`Is Not Valid`
          (set `local.XBack` Front))))
    (:`Is Not Valid`
      (set `local.XFront` Top)
      (`/Engine/EditorBlueprintResources/StandardMacros.IsValid` Back
        (:`Is Valid`
          (set `local.XBack` Back))
        (:`Is Not Valid`
          (set `local.XBack` Top)))))
  (`/Engine/EditorBlueprintResources/StandardMacros.IsValid` Right
    (:`Is Valid`
      (set `local.XRight` Right))
    (:`Is Not Valid`
      (`/Engine/EditorBlueprintResources/StandardMacros.IsValid` Front
        (:`Is Valid`
          (set `local.XRight` Front))
        (:`Is Not Valid`
          (set `local.XRight` Top)))))
  (`/Engine/EditorBlueprintResources/StandardMacros.IsValid` Left
    (:`Is Valid`
      (set `local.XLeft` Left))
    (:`Is Not Valid`
      (set `local.XLeft` Front)
      (`/Engine/EditorBlueprintResources/StandardMacros.IsValid` Front
        (:`Is Valid`
          (set `local.XLeft` Front))
        (:`Is Not Valid`
          (set `local.XLeft` Top)))))
  (if (== (`self.index`) id)
    (bind _returnvalue (`AddComponent|NODE_AddInstancedStaticMeshComponent-5` :`bManualAttachment` true))
    (`SceneComponent.K2_AttachToComponent` _returnvalue (`self.DefaultSceneRoot`) "None" "KeepRelative" "KeepRelative" "KeepRelative" true)
    (`PrimitiveComponent.SetMaterial` _returnvalue 0 (`local.XTop`))
    (`PrimitiveComponent.SetMaterial` _returnvalue 1 (`local.XBottom`))
    (`PrimitiveComponent.SetMaterial` _returnvalue 2 (`local.XFront`))
    (`PrimitiveComponent.SetMaterial` _returnvalue 3 (`local.XBack`))
    (`PrimitiveComponent.SetMaterial` _returnvalue 4 (`local.XRight`))
    (`PrimitiveComponent.SetMaterial` _returnvalue 5 (`local.XLeft`))
    (`KismetArrayLibrary.Array_Add` (`self.meshArray`) _returnvalue)))

(fn `nextLayer`
  (params (Index :type Integer))
  (bind _mesharray (`self.meshArray`))
  (bind _output (`|GetArrayItem` (`self.worldArray`) Index))
  (for _index (range (`KismetArrayLibrary.Array_Length` _mesharray))
    (`/Engine/EditorBlueprintResources/StandardMacros.IncrementInt` (`self.newLineCounter`)
      (:`  `
        (`self.checkBlock` _output (`|GetArrayItem` _mesharray _index) _index))))
  (if (`KismetStringLibrary.EqualEqual_StrStr` _output "LINEBREAK")
    (`KismetSystemLibrary.PrintString` (`KismetStringLibrary.Conv_IntToString` (`self.newLineCounter`)))
    (set `self.newLineCounter` 0)
    (set `self.x` 0)
    (bind _output_get (set `self.y` (+ (stale _output_get) 1)))
    (elif (`KismetStringLibrary.EqualEqual_StrStr` _output "LAYERBREAK")
      (set `self.x` 0)
      (set `self.y` 0)
      (bind _output_get_2 (set `self.z` (+ (stale _output_get_2) 1))))))

(fn `placeBlock`
  (params (block :type "InstancedStaticMeshComponent Object Reference") (x :type Integer) (y :type Integer) (z :type Integer))
  (`KismetSystemLibrary.PrintString` (`KismetSystemLibrary.GetDisplayName` (`PrimitiveComponent.GetMaterial` block 0)) true true (struct :`G` 0.66 :`B` 1.0 :`A` 1.0) 20.0)
  (`InstancedStaticMeshComponent.AddInstance` block (`KismetMathLibrary.MakeTransform` (`KismetMathLibrary.MakeVector` (`KismetMathLibrary.Conv_IntToDouble` (* x 200)) (`KismetMathLibrary.Conv_IntToDouble` (* y 200)) (`KismetMathLibrary.Conv_IntToDouble` (* z 200)))))
  (bind _output_get (set `self.x` (+ (stale _output_get) 1))))

(fn `scanBlocks`
  (locals (BlockArray :type "MaterialInterface Object Reference"))
  (for _index (range 59)
    (set `self.index` _index)
    (`self.createMeshes` null)
    (`self.createMeshes` "/Game/Materials/Blocks/MAT_Bedrock.MAT_Bedrock" null null null null null 1)
    (`self.createMeshes` "/Game/Materials/Blocks/MAT_Stone.MAT_Stone" null null null null null 2)
    (`self.createMeshes` "/Game/Materials/Blocks/MAT_Dirt.MAT_Dirt" null null null null null 3)
    (`self.createMeshes` "/Game/Materials/Blocks/MAT_Sand.MAT_Sand" null null null null null 4)
    (`self.createMeshes` "/Game/Materials/Blocks/MAT_Leaves.MAT_Leaves" null null null null null 5)
    (`self.createMeshes` "/Game/Materials/Blocks/MAT_TrunkTop.MAT_TrunkTop" null "/Game/Materials/Blocks/MAT_TrunkSide.MAT_TrunkSide" null null null 6)
    (`self.createMeshes` "/Game/Materials/Blocks/MAT_Wood.MAT_Wood" null null null null null 7)
    (`self.createMeshes` "/Game/Materials/Blocks/MAT_GrassTop.MAT_GrassTop" null "/Game/Materials/Blocks/MAT_GrassSide.MAT_GrassSide" null null null 8)
    (`self.createMeshes` "/Game/Materials/Blocks/MAT_TNTTop.MAT_TNTTop" null "/Game/Materials/Blocks/MAT_TNTSide.MAT_TNTSide" null null null 9)
    (`self.createMeshes` "/Game/Materials/Blocks/MAT_Rock.MAT_Rock" null null null null null 10)
    (`self.createMeshes` "/Game/Materials/Blocks/MAT_WeedsTop.MAT_WeedsTop" null "/Game/Materials/Blocks/MAT_WeedsSide.MAT_WeedsSide" null null null 11)
    (`self.createMeshes` "/Game/Materials/Blocks/MAT_FlowersTop.MAT_FlowersTop" null "/Game/Materials/Blocks/MAT_GrassSide.MAT_GrassSide" null null null 12)
    (`self.createMeshes` "/Game/Materials/Blocks/MAT_Brick.MAT_Brick" null null null null null 13)
    (`self.createMeshes` "/Game/Materials/Blocks/MAT_Roof.MAT_Roof" null null null null null 14)
    (`self.createMeshes` "/Game/Materials/Blocks/MAT_Ice.MAT_Ice" null null null null null 15)
    (`self.createMeshes` "/Game/Materials/Blocks/MAT_Wallpaper.MAT_Wallpaper" null null null null null 16)
    (`self.createMeshes` "/Game/Materials/Blocks/MAT_Trampoline.MAT_Trampoline" null null null null null 17)
    (`self.createMeshes` "/Game/Materials/Blocks/MAT_Wood.MAT_Wood" null "/Game/Materials/Blocks/MAT_LadderSide.MAT_LadderSide" null null null 18)
    (`self.createMeshes` "/Game/Materials/Blocks/MAT_Cloud.MAT_Cloud" null null null null null 19)
    (`self.createMeshes` "/Game/Materials/Blocks/MAT_Water.MAT_Water" null null null null null 20)
    (`self.createMeshes` "/Game/Materials/Blocks/MAT_Fence.MAT_Fence" null null null null null 21)
    (`self.createMeshes` "/Game/Materials/Blocks/MAT_Vines.MAT_Vines" null null null null null 22)
    (`self.createMeshes` "/Game/Materials/Blocks/MAT_Lava.MAT_Lava" null null null null null 23)
    (`self.createMeshes` "/Game/Materials/Blocks/MAT_Rock.MAT_Rock" null null null null null 24)
    (`self.createMeshes` "/Game/Materials/Blocks/MAT_Rock.MAT_Rock" null null null null null 25)
    (`self.createMeshes` "/Game/Materials/Blocks/MAT_Rock.MAT_Rock" null null null null null 26)
    (`self.createMeshes` "/Game/Materials/Blocks/MAT_Rock.MAT_Rock" null null null null null 27)
    (`self.createMeshes` "/Game/Materials/Blocks/MAT_Wood.MAT_Wood" null null null null null 28)
    (`self.createMeshes` "/Game/Materials/Blocks/MAT_Wood.MAT_Wood" null null null null null 29)
    (`self.createMeshes` "/Game/Materials/Blocks/MAT_Wood.MAT_Wood" null null null null null 30)
    (`self.createMeshes` "/Game/Materials/Blocks/MAT_Wood.MAT_Wood" null null null null null 31)
    (`self.createMeshes` "/Game/Materials/Blocks/MAT_Roof.MAT_Roof" null null null null null 32)
    (`self.createMeshes` "/Game/Materials/Blocks/MAT_Roof.MAT_Roof" null null null null null 33)
    (`self.createMeshes` "/Game/Materials/Blocks/MAT_Roof.MAT_Roof" null null null null null 34)
    (`self.createMeshes` "/Game/Materials/Blocks/MAT_Roof.MAT_Roof" null null null null null 35)
    (`self.createMeshes` "/Game/Materials/Blocks/MAT_Ice.MAT_Ice" null null null null null 36)
    (`self.createMeshes` "/Game/Materials/Blocks/MAT_Ice.MAT_Ice" null null null null null 37)
    (`self.createMeshes` "/Game/Materials/Blocks/MAT_Ice.MAT_Ice" null null null null null 38)
    (`self.createMeshes` "/Game/Materials/Blocks/MAT_Ice.MAT_Ice" null null null null null 39)
    (`self.createMeshes` "/Game/Materials/Blocks/MAT_Rock.MAT_Rock" null null null null null 40)
    (`self.createMeshes` "/Game/Materials/Blocks/MAT_Rock.MAT_Rock" null null null null null 41)
    (`self.createMeshes` "/Game/Materials/Blocks/MAT_Rock.MAT_Rock" null null null null null 42)
    (`self.createMeshes` "/Game/Materials/Blocks/MAT_Rock.MAT_Rock" null null null null null 43)
    (`self.createMeshes` "/Game/Materials/Blocks/MAT_Wood.MAT_Wood" null null null null null 44)
    (`self.createMeshes` "/Game/Materials/Blocks/MAT_Wood.MAT_Wood" null null null null null 45)
    (`self.createMeshes` "/Game/Materials/Blocks/MAT_Wood.MAT_Wood" null null null null null 46)
    (`self.createMeshes` "/Game/Materials/Blocks/MAT_Wood.MAT_Wood" null null null null null 47)
    (`self.createMeshes` "/Game/Materials/Blocks/MAT_Roof.MAT_Roof" null null null null null 48)
    (`self.createMeshes` "/Game/Materials/Blocks/MAT_Roof.MAT_Roof" null null null null null 49)
    (`self.createMeshes` "/Game/Materials/Blocks/MAT_Roof.MAT_Roof" null null null null null 50)
    (`self.createMeshes` "/Game/Materials/Blocks/MAT_Roof.MAT_Roof" null null null null null 51)
    (`self.createMeshes` "/Game/Materials/Blocks/MAT_Ice.MAT_Ice" null null null null null 52)
    (`self.createMeshes` "/Game/Materials/Blocks/MAT_Ice.MAT_Ice" null null null null null 53)
    (`self.createMeshes` "/Game/Materials/Blocks/MAT_Ice.MAT_Ice" null null null null null 54)
    (`self.createMeshes` "/Game/Materials/Blocks/MAT_Ice.MAT_Ice" null null null null null 55)
    (`self.createMeshes` "/Game/Materials/Blocks/MAT_Roof.MAT_Roof" null null null null null 56)
    (`self.createMeshes` "/Game/Materials/Blocks/MAT_Tiles.MAT_Tiles" null null null null null 57)
    (`self.createMeshes` "/Game/Materials/Blocks/MAT_Glass.MAT_Glass" null null null null null 58)
    (`self.createMeshes` "/Game/Materials/Blocks/MAT_Water.MAT_Water" null null null null null 59)
    (`self.createMeshes` "/Game/Materials/Blocks/MAT_Water.MAT_Water" null null null null null 60)
    (`self.createMeshes` "/Game/Materials/Blocks/MAT_Water.MAT_Water" null null null null null 61)
    (`self.createMeshes` "/Game/Materials/Blocks/MAT_Lava.MAT_Lava" null null null null null 62)
    (`self.createMeshes` "/Game/Materials/Blocks/MAT_Lava.MAT_Lava" null null null null null 63)
    (`self.createMeshes` "/Game/Materials/Blocks/MAT_Lava.MAT_Lava" null null null null null 64))
  (bind _output_get (set `self.worldArray` (`KismetStringLibrary.ParseIntoArray` (`FileBlueprintFunctionLibrary.FileLoadString` "/Converter/world.out") "|")))
  (set `self.x` 0)
  (set `self.y` 0)
  (set `self.z` 0)
  (`KismetSystemLibrary.PrintString` (`KismetStringLibrary.Conv_IntToString` (`KismetArrayLibrary.Array_Length` _output_get))))

(fn `UserConstructionScript`)